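; Looping spawner actor that plays stylized water splash effects with a water decal at its location, scaled in intensity by its Level variable.
; BeginPlay waits a Level-based delay, then the self-calling Again event repeats the spawn every 4.5 seconds, passing Level to BP_Water_Decal.
; Levels 1 and 2 each play one splash system; level 3 staggers four alternating splashes at random offsets, one per quadrant.
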(event `Again`
  (bind _returnvalue (`self.K2_GetActorLocation`))
  (`KismetSystemLibrary.Delay` 4.5)
  (`|SpawnActorFromClass` "/Game/Art/Stylized_VFX_StPack/Blueprints/BP_Water_Decal.BP_Water_Decal_C" (`KismetMathLibrary.MakeTransform` (`self.K2_GetActorLocation`)) "Undefined" "OverrideRootScale" null (`self.Level`) null :!label _label)
  (switch `int` (`self.Level`)
    (:`1`
      (`NiagaraFunctionLibrary.SpawnSystemAtLocation` "/Game/Art/Stylized_VFX_StPack/Particles/P_Splash_01.P_Splash_01" _returnvalue)
      (`self.Again` :!label _label_2))
    (:`2`
      (`NiagaraFunctionLibrary.SpawnSystemAtLocation` "/Game/Art/Stylized_VFX_StPack/Particles/P_Splash_02.P_Splash_02" _returnvalue)
      (goto _label_2))
    (:`3`
      (`NiagaraFunctionLibrary.SpawnSystemAtLocation` "/Game/Art/Stylized_VFX_StPack/Particles/P_Splash_02.P_Splash_02" (+ (`self.K2_GetActorLocation`) (`KismetMathLibrary.MakeVector` (`KismetMathLibrary.RandomFloatInRange` 30.0 60.0) (`KismetMathLibrary.RandomFloatInRange` 30.0 60.0))))
      (`|ExecutionSequence`
        (:`then_0`
          (goto _label_2))
        (:`then_1`
          (`KismetSystemLibrary.Delay` 0.25)
          (`NiagaraFunctionLibrary.SpawnSystemAtLocation` "/Game/Art/Stylized_VFX_StPack/Particles/P_Splash_01.P_Splash_01" (+ (`self.K2_GetActorLocation`) (`KismetMathLibrary.MakeVector` (`KismetMathLibrary.RandomFloatInRange` -60.0 -30.0) (`KismetMathLibrary.RandomFloatInRange` 30.0 60.0))))
          (`KismetSystemLibrary.Delay` 0.15)
          (`NiagaraFunctionLibrary.SpawnSystemAtLocation` "/Game/Art/Stylized_VFX_StPack/Particles/P_Splash_02.P_Splash_02" (+ (`self.K2_GetActorLocation`) (`KismetMathLibrary.MakeVector` (`KismetMathLibrary.RandomFloatInRange` 30.0 60.0) (`KismetMathLibrary.RandomFloatInRange` -60.0 -30.0))))
          (`KismetSystemLibrary.Delay` 0.2)
          (`NiagaraFunctionLibrary.SpawnSystemAtLocation` "/Game/Art/Stylized_VFX_StPack/Particles/P_Splash_01.P_Splash_01" (+ (`self.K2_GetActorLocation`) (`KismetMathLibrary.MakeVector` (`KismetMathLibrary.RandomFloatInRange` -60.0 -30.0) (`KismetMathLibrary.RandomFloatInRange` -60.0 -30.0)))))))))

(event `self.ReceiveBeginPlay`
  (`KismetSystemLibrary.Delay` (* (`self.Level`) 1.5))
  (goto _label))

(fn `UserConstructionScript`)