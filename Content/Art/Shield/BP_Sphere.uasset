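; BP_Sphere is a physics sphere that slows and dissolves away when it overlaps a BP_Shield actor.
; On overlap it swaps in a dynamic dissolve material and stores a fraction of its current velocity.
; Tick reapplies that reduced velocity every frame while dissolving, so the sphere drifts at constant speed.
; The Disolve timeline drives the material's Progress parameter and destroys the actor when finished.
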(event `self.ReceiveActorBeginOverlap`
  (params (OtherActor :type "Actor Object Reference"))
  (bind _sphere (`self.Sphere`))
  (if (== (`GameplayStatics.GetObjectClass` OtherActor) "/Game/Art/Shield/BP_Shield.BP_Shield_C")
    (bind _returnvalue (`KismetMaterialLibrary.CreateDynamicMaterialInstance` "/Game/Art/Shield/M_Dissolve_Inst.M_Dissolve_Inst"))
    (`PrimitiveComponent.SetMaterial` (`self.Sphere`) 0 _returnvalue)
    (set `self.IsDisolving` true)
    (bind _returnvalue_2 (`PrimitiveComponent.GetPhysicsLinearVelocity` _sphere "None"))
    (bind _output_get (set `self.Force` (/ _returnvalue_2 5.0)))
    (`PrimitiveComponent.SetPhysicsLinearVelocity` _sphere _output_get false "None")
    (bind (_direction _value) (`Timeline|Disolve`)
      (:`Update`
        (`MaterialInstanceDynamic.SetScalarParameterValue` _returnvalue "Progress" _value))
      (:`Finished`
        (`self.K2_DestroyActor`)))))

(event `self.ReceiveTick`
  (params (DeltaSeconds :type "Float (single-precision)"))
  (if (`self.IsDisolving`)
    (`PrimitiveComponent.SetPhysicsLinearVelocity` (`self.Sphere`) (`self.Force`) false "None")))

(fn `UserConstructionScript`)