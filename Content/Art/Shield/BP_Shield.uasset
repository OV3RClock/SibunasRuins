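; BP_Shield is a shield actor that dissolves BP_Sphere projectiles overlapping it and shows a material hit effect.
; On overlap it passes an outward direction to the sphere's dissolve and feeds the sphere's position and a timeline value into one hit slot on a dynamic material.
; Show and Hide toggle query collision and run opposing timelines that drive scale and spawn fade, while HideInstant skips the animation.
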(event `self.ReceiveBeginPlay`
  (bind _returnvalue (`KismetMaterialLibrary.CreateDynamicMaterialInstance` "/Game/Art/Shield/M_Shield_Inst.M_Shield_Inst"))
  (bind _output_get (set `self.ShieldMaterial` _returnvalue))
  (`PrimitiveComponent.SetMaterial` (`self.Mesh`) 0 _output_get))

(event `self.ReceiveActorBeginOverlap`
  (params (OtherActor :type "Actor Object Reference"))
  (bind _shieldmaterial (`self.ShieldMaterial`))
  ;[1 1 1] Hit projectile
  (if (== (`GameplayStatics.GetObjectClass` OtherActor) "/Game/Art/Shield/BP_Sphere.BP_Sphere_C")
    (bind _asbp_sphere (cast `/Game/Art/Shield/BP_Sphere` OtherActor))
    (if (not (`/Game/Art/Shield/BP_Sphere.IsDisolving` _asbp_sphere))
      (`/Game/Art/Shield/BP_Sphere.DisolveAndDestroy` _asbp_sphere (`KismetMathLibrary.Normal` (- (`self.K2_GetActorLocation` _asbp_sphere) (`self.K2_GetActorLocation`))))
      (`MaterialInstanceDynamic.SetVectorParameterValue` _shieldmaterial "HitPosition1" (`KismetMathLibrary.Conv_VectorToLinearColor` (`SceneComponent.K2_GetComponentLocation` (`Actor.RootComponent` OtherActor))))
      (bind (_direction _hitvalue) (`Timeline|ShieldMatHit` :!via `PlayFromStart`)
        (:`Update`
          (`MaterialInstanceDynamic.SetScalarParameterValue` _shieldmaterial "HitValue1" (* _hitvalue 1.0)))))))

(event `Show`
  ;[1 1 1] Show
  (`SceneComponent.SetVisibility` (`self.Mesh`) true false)
  (`PrimitiveComponent.SetCollisionEnabled` (`self.Mesh`) "QueryOnly")
  (bind (_direction _spawnvalue _scale) (`Timeline|Spawn` :!via `PlayFromStart` :!label _label)
    (:`Update`
      (`self.SetActorScale3D` (`KismetMathLibrary.Conv_DoubleToVector` _scale))
      (`MaterialInstanceDynamic.SetScalarParameterValue` (`self.ShieldMaterial`) "SpawnFade" _spawnvalue)
      ;[1 1 1] Hide
      (bind (_direction_2 _spawnvalue_2 _scale_2) (`Timeline|Despawn` :!via `Stop` :!label _label_2)
        (:`Update`
          (`self.SetActorScale3D` (`KismetMathLibrary.Conv_DoubleToVector` _scale_2))
          (`MaterialInstanceDynamic.SetScalarParameterValue` (`self.ShieldMaterial`) "SpawnFade" _spawnvalue_2)
          (goto _label :!via `Stop`))
        (:`Finished`
          (`SceneComponent.SetVisibility` (`self.Mesh`) false false))))))

(event `Hide`
  ;[1 1 1] Hide
  (`PrimitiveComponent.SetCollisionEnabled` (`self.Mesh`) "NoCollision")
  (goto _label_2 :!via `PlayFromStart`))

(event `HideInstant`
  ;[1 1 1] Hide Instant
  (`SceneComponent.SetVisibility` (`self.Mesh`) false false)
  (`PrimitiveComponent.SetCollisionEnabled` (`self.Mesh`) "NoCollision"))

(fn `UserConstructionScript`)