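; Goblin enemy Blueprint that plays a dissolve death effect when it takes damage, which it applies to itself on BeginPlay.
; The first hit sets IsDead and GetHit, then swaps the mesh to a dynamic instance of MI_Dissolve2.
; A Timeline animates that material's Offset scalar and stops itself at the end value.
; DestroyActor is wired to Finished, which that manual Stop can prevent from firing.
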(event `self.ReceiveBeginPlay`
  (`GameplayStatics.ApplyDamage` self 1.0))

(event `self.ReceiveAnyDamage`
  (params (Damage :type "Float (single-precision)") (DamageType :type "DamageType Object Reference") (InstigatedBy :type "Controller Object Reference") (DamageCauser :type "Actor Object Reference"))
  (if (not (`self.GetHit`))
    (set `self.IsDead` true)
    (bind _returnvalue (`KismetMaterialLibrary.CreateDynamicMaterialInstance` "/Game/Art/Dissolve/MI_Dissolve2.MI_Dissolve2"))
    (set `self.GetHit` true)
    (`PrimitiveComponent.SetMaterial` (`self.SM_EnemyGoblin`) 0 _returnvalue)
    (bind (_direction _dissolve) (`Timeline|Timeline` :!via `PlayFromStart` :!label _label)
      (:`Update`
        (bind _returnvalue_2 (`KismetMathLibrary.Lerp` -0.7 1.3 _dissolve))
        (`MaterialInstanceDynamic.SetScalarParameterValue` _returnvalue "Offset" _returnvalue_2)
        (if (== _returnvalue_2 1.3)
          (goto _label :!via `Stop`)))
      (:`Finished`
        (`self.K2_DestroyActor`)))))

(fn `UserConstructionScript`)